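; BP_Door_V2 is a door that swings open automatically when an actor overlaps its Trigger volume and closes when the overlap ends.
; On overlap, a dot product of the actor's and door's forward vectors picks the swing direction from the actor's facing.
; The SwingDoor timeline drives a yaw lerp to a quarter turn either way, and reverses on end overlap.
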(event OnComponentBeginOverlap(Trigger)
  (params (OverlappedComponent :type Primitive%20Component%20Object%20Reference) (OtherActor :type Actor%20Object%20Reference) (OtherComp :type Primitive%20Component%20Object%20Reference) (OtherBodyIndex :type Integer) (bFromSweep :type Boolean) (SweepResult :type Hit%20Result%20Structure%20%28by%20ref%29))
  (bind _door (Variables|Default|GetDoor))
  (Variables|Default|SetFacingCharacter (>= (Math|Vector|DotProduct (Transformation|GetActorForwardVector OtherActor) (Transformation|GetActorForwardVector (Components|GetOwner (Variables|Default|GetDefaultSceneRoot)))) 0.0))
  (bind _swingdoor (Timeline|SwingDoor Play)
    (:Update
      (if (Variables|Default|GetFacingCharacter)
        (Transformation|SetRelativeRotation _door (Math|Rotator|MakeRotator 0.0 0.0 (Math|Float|Lerp 0.0 9e+01 (.z _swingdoor))) false false)
        (else
          (Transformation|SetRelativeRotation _door (Math|Rotator|MakeRotator 0.0 0.0 (Math|Float|Lerp 0.0 -9e+01 (.z _swingdoor))) false false))))))

(event OnComponentEndOverlap(Trigger)
  (params (OverlappedComponent :type Primitive%20Component%20Object%20Reference) (OtherActor :type Actor%20Object%20Reference) (OtherComp :type Primitive%20Component%20Object%20Reference) (OtherBodyIndex :type Integer))
  (bind _door (Variables|Default|GetDoor))
  (bind _swingdoor (Timeline|SwingDoor Reverse)
    (:Update
      (if (Variables|Default|GetFacingCharacter)
        (Transformation|SetRelativeRotation _door (Math|Rotator|MakeRotator 0.0 0.0 (Math|Float|Lerp 0.0 9e+01 (.z _swingdoor))) false false)
        (else
          (Transformation|SetRelativeRotation _door (Math|Rotator|MakeRotator 0.0 0.0 (Math|Float|Lerp 0.0 -9e+01 (.z _swingdoor))) false false))))))

(fn ConstructionScript)